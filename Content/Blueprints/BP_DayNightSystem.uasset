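; Day-night system actor that animates a directional light to simulate passing time.
; When activated, BeginPlay waits briefly, enables Tick and starts a timeline at a configurable play rate.
; The timeline drives the light's yaw and intensity, plus ShadeContrast in a cel-shading material parameter collection so shading follows brightness.
; Tick separately adds world pitch rotation to the light, scaled by TimeRate.
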(event EventBeginPlay
  (bind _activatedaytimesystem (Variables|Default|GetActivateDaytimeSystem))
  (if _activatedaytimesystem
    (Utilities|FlowControl|Delay 0.2)
    (Actor|Tick|SetActorTickEnabled _activatedaytimesystem)
    (bind _output_get (Variables|Default|SetDirectionLightComponent (Variables|/Script/Engine.Light|GetLightComponent (Variables|Default|GetDirectionalLight))))
    (Variables|Default|SetCurrentLightIntensity (Variables|/Script/Engine.LightComponentBase|GetIntensity _output_get))
    (Components|Timeline|SetPlayRate (Variables|Default|GetLightTimeline) (Variables|Default|GetPlayRate))
    (Utilities|IsValid (Variables|Default|GetDirectionLightComponent)
      (:Is%20Valid
        (bind (_direction _newtrack_0 _newtrack_1) (Timeline|LightTimeline PlayFromStart)
          (:Update
            (Transformation|SetRelativeRotation (Variables|Default|GetDirectionLightComponent) (Math|Rotator|MakeRotator (.roll (Variables|/Script/Engine.SceneComponent|GetRelativeRotation (Variables|Default|GetDirectionLightComponent))) (.pitch (Variables|/Script/Engine.SceneComponent|GetRelativeRotation (Variables|Default|GetDirectionLightComponent))) (Math|Float|Lerp 0.0 3.6e+02 _newtrack_1)) false false)
            (Rendering|Components|Light|SetIntensity (Variables|Default|GetDirectionLightComponent) (Math|Float|Lerp (Variables|Default|GetMinLightIntensity) (Variables|Default|GetMaxLightIntensity) _newtrack_0))
            (Rendering|Material|SetScalarParameterValue (Variables|Default|GetCelShadingParamCollection) (Utilities|String|StringToName "ShadeContrast") (Math|Float|Lerp 0.35 1.0 _newtrack_0) :!class /Script/Engine.KismetMaterialLibrary)))))))

(event Collision|EventActorBeginOverlap
  (params (OtherActor :type Actor%20Object%20Reference)))

(event EventTick
  (params (DeltaSeconds :type Float%20%28single-precision%29))
  (Transformation|AddWorldRotation (Variables|/Script/Engine.Light|GetLightComponent (Variables|Default|GetDirectionalLight)) (Math|Rotator|MakeRotator 0.0 (* DeltaSeconds (Variables|Default|GetTimeRate)) 0.0) false false))

(fn ConstructionScript)